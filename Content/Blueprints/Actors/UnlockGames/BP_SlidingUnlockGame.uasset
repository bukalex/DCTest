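; Sliding unlock minigame actor that unlocks a drive once a slider has been moved far enough.
; Each sprite move on the Slider measures the distance between Connector and Body against UnlockDistance.
; Reaching that threshold fires once, locking the Slider's translation and calling UnlockDrive.
; Tick keeps the Slider's world scale matched to the Body's.
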(event `self.ReceiveTick`
  (params (DeltaSeconds :type "Float (single-precision)"))
  (`SceneComponent.SetWorldScale3D` (`self.Slider`) (`SceneComponent.K2_GetComponentScale` (`self.Body`))))

(event `self.Slider.OnSpriteMoved`
  (if (>= (`KismetMathLibrary.Vector_Distance` (`SceneComponent.K2_GetComponentLocation` (`self.Connector`)) (`SceneComponent.K2_GetComponentLocation` (`self.Body`))) (`self.UnlockDistance`))
    (`/Engine/EditorBlueprintResources/StandardMacros.DoOnce` false
      (:`Completed`
        (`|ExecutionSequence`
          (:`then_0`
            (set `DraggableSpriteComponent.bLockTranslation` true (`self.Slider`)))
          (:`then_1`
            (`self.UnlockDrive`)))))))

(fn `UserConstructionScript`)