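; BP_CapUnlockGame is an unlock minigame in which a drive is unlocked by separating its cap from the body.
; Whenever the cap or body sprite moves, it measures the cap's offset along the body's local X axis against a minimum distance.
; The first time that threshold is reached, it locks the body's movement, ignores its collision, hides the cap and calls UnlockDrive.
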(event `self.LineTraceCap.OnSpriteMoved`
  (bind _drivebody (`self.DriveBody`))
  (bind _returnvalue_x (`KismetMathLibrary.BreakVector` (`KismetMathLibrary.InverseTransformLocation` (`SceneComponent.K2_GetComponentToWorld` (`self.DriveBody`)) (`SceneComponent.K2_GetComponentLocation` (`self.CapEmpty`)))))
  (if (>= (`KismetMathLibrary.Abs` _returnvalue_x) (`self.MinCapOffset`)) :!label _label
    (`/Engine/EditorBlueprintResources/StandardMacros.DoOnce` false
      (:`Completed`
        (`|ExecutionSequence`
          (:`then_0`
            (set `DraggableSpriteComponent.bLockTranslation` true _drivebody)
            (set `DraggableSpriteComponent.bLockRotation` true _drivebody)
            (`PrimitiveComponent.SetCollisionResponseToAllChannels` _drivebody "ECR_Ignore"))
          (:`then_1`
            (`SceneComponent.SetHiddenInGame` (`self.CapEmpty`) true true))
          (:`then_2`
            (`self.UnlockDrive`)))))))

(event `self.DriveBody.OnSpriteMoved`
  (goto _label))

(fn `UserConstructionScript`)