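; Unlock mini-game actor in which rotating a cap relative to its body unlocks a drive.
; Movement of either the Cap or Body sprite runs a shared check on the dot product of their up vectors.
; Once they are at least 90 degrees apart, a DoOnce locks both parts' rotation and calls UnlockDrive.
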(event `self.Cap.OnSpriteMoved`
  (if (<= (`KismetMathLibrary.Dot_VectorVector` (`SceneComponent.GetUpVector` (`self.Body`)) (`SceneComponent.GetUpVector` (`self.Cap`))) 0.0) :!label _label
    (`/Engine/EditorBlueprintResources/StandardMacros.DoOnce` false
      (:`Completed`
        (`|ExecutionSequence`
          (:`then_0`
            (set `DraggableSpriteComponent.bLockRotation` true (`self.Cap`)))
          (:`then_1`
            (set `DraggableSpriteComponent.bLockRotation` true (`self.Body`)))
          (:`then_2`
            (`self.UnlockDrive`)))))))

(event `self.Body.OnSpriteMoved`
  (goto _label))

(fn `UserConstructionScript`)